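; BP_Dome is a dome that carries a player-controlled turret along its upper arc and relays fire input to it.
; BeginPlay finds the BP_Turret and reads the sphere's bounds as the arc's width and height.
; Rotate input steps an angle clamped to a half circle, which Tick converts with sine and cosine into turret position and Atan2-based outward roll.
; Shoot input calls the turret's Shoot on start and while ongoing.
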(event Input|EnhancedActionEvents|EnhancedInputActionIA_Shoot
  (params (ActionValue :type Boolean) (ElapsedSeconds :type Float%20%28double-precision%29) (TriggeredSeconds :type Float%20%28double-precision%29) (InputAction :type Input%20Action%20Object%20Reference :default "/Game/ThirdPerson/Input/Actions/IA_Shoot.IA_Shoot"))
  ;[1 0.3824 0] Shoot_Event
  (:Started
    (Default|Shoot (Variables|BP_Ref|GetBP_Turret_Ref) :!label _label))
  (:Ongoing
    (goto _label)))

(event Input|EnhancedActionEvents|EnhancedInputActionIA_Rotate_Turret
  (params (ActionValue :type Float%20%28double-precision%29) (ElapsedSeconds :type Float%20%28double-precision%29) (TriggeredSeconds :type Float%20%28double-precision%29) (InputAction :type Input%20Action%20Object%20Reference :default "/Game/ThirdPerson/Input/Actions/IA_Rotate_Turret.IA_Rotate_Turret"))
  ;[0 0.7608 1] Event_Move_Turret_Around_Shield
  (if (> ActionValue 0.0)
    (Variables|Turret_Rotation|SetTurret_Angle_Rotation (Math|Float|Clamp(Float) (+ (Variables|Turret_Rotation|GetTurret_Angle_Rotation) 1.0) -9e+01 9e+01))
    (elif (< ActionValue 1.0)
      (Variables|Turret_Rotation|SetTurret_Angle_Rotation (Math|Float|Clamp(Float) (- (Variables|Turret_Rotation|GetTurret_Angle_Rotation) 1.0) -9e+01 9e+01)))))

(event EventBeginPlay
  (bind _sphere (Variables|Default|GetSphere))
  (bind _boxextent (Collision|GetComponentBounds _sphere))
  ;[0 0 0] Event_BeginPlay
  (Variables|Default|SetCan_Shoot_?? false)
  (bind _returnvalue (Actor|GetActorOfClass "/Game/Dome/BP_Turret.BP_Turret_C"))
  (Variables|BP_Ref|SetBP_Turret_Ref _returnvalue)
  (Variables|Dome_Parameters|SetWidth (.y _boxextent))
  (Variables|DomeParameters|SetHeight (.z _boxextent)))

(event EventTick
  (params (DeltaSeconds :type Float%20%28single-precision%29))
  (bind _turret_angle_rotation (Variables|Turret_Rotation|GetTurret_Angle_Rotation))
  (bind _returnvalue (Math|Float|Clamp(Float) _turret_angle_rotation -9e+01 9e+01))
  ;[0.08082 1 0] Rotate_Turret_Arround_Shield_With_Find_Look_At_Rotation
  (bind _bp_turret_ref (Variables|BP_Ref|GetBP_Turret_Ref)
    (:then
      (bind _output_get (Variables|TurretRotation|SetTurret_Angle_XRota (* (Math|Trig|Sin(Degrees) _returnvalue) (Variables|Dome_Parameters|GetWidth))))
      (bind _output_get_2 (Variables|TurretRotation|SetTurret_Angle_ZRota (* (Math|Trig|Cos(Degrees) _returnvalue) (Variables|DomeParameters|GetHeight))))
      (Transformation|SetActorLocation _bp_turret_ref (+ (Math|Vector|MakeVector 0.0 _output_get _output_get_2) (Transformation|GetWorldLocation (Variables|Default|GetSphere))) false false)
      (Transformation|SetActorRotation (Variables|BP_Ref|GetBP_Turret_Ref) (Math|Rotator|MakeRotator (|(R*(180/PI)) (Math|Trig|Atan2(Radians) (Variables|TurretRotation|GetTurret_Angle_XRota) (Variables|TurretRotation|GetTurret_Angle_ZRota)) (Math|Trig|GetPI)) 0.0 0.0)))
    (:else)))

(fn ConstructionScript)