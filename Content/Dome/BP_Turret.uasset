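; BP_Turret is a turret that fires either a basic shot or a laser, chosen by an EShootType switch in its Shoot event.
; Basic shots spawn a BP_Bullet at the Arrow component's transform.
; Laser shots debug-draw a forward sphere trace and spawn a Niagara laser effect, but the trace result is unused.
; The BP_Dome reference cached at BeginPlay only gates the laser through a validity check.
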(event `self.ReceiveBeginPlay`
  ;[0 0 0] Event_BeginPlay
  (bind _returnvalue (`GameplayStatics.GetActorOfClass` "/Game/Dome/BP_Dome.BP_Dome_C"))
  (set `self.BP_Dome_Ref` _returnvalue))

(event `Shoot`
  ;[1 0 0] Choose_Shoot_Type
  (switch `/Game/Dome/E_Shoot_Type` (`self.E_Shoot_Type`)
    (:`NewEnumerator0`
      (`self.Basic_Shoot`))
    (:`NewEnumerator1`
      (`self.Laser_Shoot`))))

(event `Basic_Shoot`
  (bind (_returnvalue_location _returnvalue_rotation) (`KismetMathLibrary.BreakTransform` (`SceneComponent.K2_GetComponentToWorld` (`self.Arrow`))))
  ;[1 0.8744 0] Basic_Shoot_Event
  (`|SpawnActorFromClass` "/Game/Dome/BP_Bullet.BP_Bullet_C" (`KismetMathLibrary.MakeTransform` _returnvalue_location _returnvalue_rotation) "Undefined" "MultiplyWithRoot" null null))

(event `Laser_Shoot`
  (bind _arrow (`self.Arrow`))
  (bind _arrow_2 (`self.Arrow`))
  (bind _returnvalue (`SceneComponent.K2_GetComponentLocation` _arrow))
  ;[1 0.3622 0] Laser_Shoot_Event
  (`self.BP_Dome_Ref`
    (:`then`
      (`KismetSystemLibrary.SphereTraceSingle` :`Start` _returnvalue :`End` (+ _returnvalue (* (`SceneComponent.GetForwardVector` _arrow) 500.0)) :`Radius` 35.0 :`TraceChannel` "TraceTypeQuery1" :`DrawDebugType` "ForDuration")
      (`NiagaraFunctionLibrary.SpawnSystemAtLocation` (`NiagaraComponent.GetAsset` (`self.NS_Laser`)) (`SceneComponent.K2_GetComponentLocation` _arrow_2) (`SceneComponent.K2_GetComponentRotation` _arrow_2)))
    (:`else`)))

(fn `UserConstructionScript`)